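; Enemy spawner actor that spawns waves of Brute and Grunt enemies when its SpawnWave event is called.
; Per-wave lookup maps set how many of each type fill the spawn list, until CurrentWave reaches MaxWaves and a cleared message prints.
; Enemies always spawn from the actor's location in stepped X offsets that rise every third spawn, each incrementing ThirdPersonGameMode's EnemiesAlive count.
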(event `SpawnWave`
  (if (< (`self.CurrentWave`) (`self.MaxWaves`))
    (`KismetArrayLibrary.Array_Clear` (`self.EnemiesToSpawn`))
    (for _ (range 1 (+ (`BlueprintMapLibrary.Map_Find` (`self.BrutesWaveInformation`) (`self.CurrentWave`)) 1))
      (`KismetArrayLibrary.Array_Add` (`self.EnemiesToSpawn`) "/Game/ThirdPersonBP/ThirdPersonBP/Blueprints/BruteEnemy.BruteEnemy_C"))
    (for _ (range 1 (+ (`BlueprintMapLibrary.Map_Find` (`self.GruntsWaveInformation`) (`self.CurrentWave`)) 1))
      (`KismetArrayLibrary.Array_Add` (`self.EnemiesToSpawn`) "/Game/ThirdPersonBP/ThirdPersonBP/Blueprints/GruntEnemy.GruntEnemy_C"))
    (set `self.LocationToSpawn` (`self.K2_GetActorLocation`))
    (for (_array_element _array_index) (`self.EnemiesToSpawn`)
      (`|SpawnActorFromClass` _array_element (`KismetMathLibrary.Conv_VectorToTransform` (`self.LocationToSpawn`)) "AlwaysSpawn" "OverrideRootScale" null null)
      (bind _asthird_person_game_mode (cast `/Game/ThirdPersonBP/ThirdPersonBP/Blueprints/ThirdPersonGameMode` (`GameplayStatics.GetGameMode`)))
      (`/Engine/EditorBlueprintResources/StandardMacros.IncrementInt` (`/Game/ThirdPersonBP/ThirdPersonBP/Blueprints/ThirdPersonGameMode.EnemiesAlive` _asthird_person_game_mode)
        (:`  `
          (if (== (mod _array_index 3) 0)
            (set `self.LocationToSpawn` (+ (`self.LocationToSpawn`) (-60.0 0.0 20.0)))
            (else
              (set `self.LocationToSpawn` (+ (`self.LocationToSpawn`) (20.0 0.0 0.0))))))))
    (else
      (`KismetSystemLibrary.PrintString` "All Waves cleared"))))

(fn `UserConstructionScript`)